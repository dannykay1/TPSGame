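; Instant-hit weapon Blueprint that plays fire and reload animation montages on the character that owns it.
; Both play events cast the owner to CharacterBase and choose the ironsights or hip montage from its IsAiming state.
; A shared PlayMontage event stops the character's mesh component before playing the chosen montage on it.
; The graph holds only this animation logic, with no hit or damage handling.
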(event `self.PlayFireAnimMontage`
  (bind _ascharacter_base (cast `CharacterBase` (`self.GetOwner`)))
  (if (`CharacterBase.bIsAiming` _ascharacter_base)
    (bind _mesh (`Character.Mesh` _ascharacter_base))
    (`self.PlayMontage` _mesh (`self.FireMontageIronsights`))
    (else
      (`self.PlayMontage` _mesh (`self.FireMontageHip`)))))

(event `PlayMontage`
  (params (MeshComponent :type "SkeletalMeshComponent Object Reference") (MontageToPlay :type "AnimMontage Object Reference"))
  (`SkeletalMeshComponent.Stop` MeshComponent)
  (`|PlayMontage` MeshComponent MontageToPlay))

(event `self.PlayReloadAnimMontage`
  (bind _ascharacter_base (cast `CharacterBase` (`self.GetOwner`)))
  (if (`CharacterBase.bIsAiming` _ascharacter_base)
    (bind _mesh (`Character.Mesh` _ascharacter_base))
    (`self.PlayMontage` _mesh (`self.ReloadMontageIronsights`))
    (else
      (`self.PlayMontage` _mesh (`self.ReloadMontageHip`)))))

(fn `UserConstructionScript`)