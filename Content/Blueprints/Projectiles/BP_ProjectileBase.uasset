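; BP_ProjectileBase is a base projectile Blueprint that child projectiles extend through an empty OnCollision hook.
; On BeginPlay it ignores its owner during movement and sets a fallback lifespan.
; The first hit on a non-owner actor calls OnCollision, disables collision, hides the mesh and resets the lifespan, so the actor lingers briefly before being destroyed.
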(event `self.ReceiveBeginPlay`
  (`PrimitiveComponent.IgnoreActorWhenMoving` (`self.CollisionComp`) (`self.GetOwner`) true)
  (`self.SetLifeSpan` 30.0))

(event `self.CollisionComp.OnComponentHit`
  (params (HitComponent :type "PrimitiveComponent Object Reference") (OtherActor :type "Actor Object Reference") (OtherComp :type "PrimitiveComponent Object Reference") (NormalImpulse :type "Vector Structure") (Hit :type "HitResult Structure (by ref)"))
  (if (!= OtherActor (`self.GetOwner`))
    (`/Engine/EditorBlueprintResources/StandardMacros.DoOnce` false
      (:`Completed`
        (`self.OnCollision`) ; Implement in child blueprints
        (`PrimitiveComponent.SetCollisionEnabled` (`self.CollisionComp`) "NoCollision")
        (`SceneComponent.SetHiddenInGame` (`self.StaticMesh`) true false)
        (`self.SetLifeSpan` 10.0)))))

(event `OnCollision`
  ;[1 1 1] Implement in child blueprints
)

(fn `UserConstructionScript`)